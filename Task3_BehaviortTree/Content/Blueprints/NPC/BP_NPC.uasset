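; BP_NPC is an NPC Blueprint with helpers for patrolling, enemy detection and firing.
; GetNextPoint steps through PatrolPoints, though its index can reach the array length before resetting, and IsLastPoint tests for the final point.
; GetNearEnemy returns Enemy, set to the last ThirdPersonCharacter found overlapping the Box and not cleared when none is found.
; OnFire is a placeholder that prints red debug text and decrements AmmoCount without checking it.
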(event Custom|OnFire
  (Development|PrintString "Tra-ta-ta" true true "(R=1.000000,G=0.000000,B=0.000000,A=1.000000)")
  (Math|Integer|DecrementInt (Variables|Default|GetAmmoCount)))

(event EventBeginPlay)

(fn ConstructionScript)

(fn GetNextPoint
  (if (< (Variables|Default|GetNextPointIndex) (Utilities|Array|Length (Variables|Default|GetPatrolPoints)))
    (Math|Integer|IncrementInt (Variables|Default|GetNextPointIndex)
      (:%20%20
        _))
    (else
      (Variables|Default|SetNextPointIndex 0)))
  (return (Utilities|Array|Get(acopy) (Variables|Default|GetPatrolPoints) (Variables|Default|GetNextPointIndex))))

(fn IsLastPoint
  (params (TargetPoint :type Target%20Point%20Object%20Reference))
  (bind _patrolpoints (Variables|Default|GetPatrolPoints))
  (return (== TargetPoint (Utilities|Array|Get(acopy) _patrolpoints (- (Utilities|Array|Length _patrolpoints) 1)))))

(fn GetNearEnemy
  (for _array_element (Collision|GetOverlappingActors (Variables|Default|GetBox) "/Game/ThirdPersonBP/Blueprints/ThirdPersonCharacter.ThirdPersonCharacter_C" :!class /Script/Engine.PrimitiveComponent)
    (bind _asthird_person_character (Utilities|Casting|CastToThirdPersonCharacter _array_element))
    (LocalVariables|SetEnemy _asthird_person_character))
  (return (LocalVariables|GetEnemy)))